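; Player wagon pawn that drives as a Chaos wheeled vehicle, rides spline rails and glides by parachute, with jump, turbo, missiles, pickups, HUD and damage.
; A VehicleMode switch routes Enhanced Input and Tick between Wheels and Rail.
; Overlapping a "Rail"-tagged spline disables physics and moves the mesh by spline distance; jumping or reaching the end restores physics with an exit impulse.
; The parachute applies lift, glide and steering forces while banking a visual mesh and camera.
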(event OnComponentBeginOverlap(RailDetector)
  (params (OverlappedComponent :type Primitive%20Component%20Object%20Reference) (OtherActor :type Actor%20Object%20Reference) (OtherComp :type Primitive%20Component%20Object%20Reference) (OtherBodyIndex :type Integer) (bFromSweep :type Boolean) (SweepResult :type Hit%20Result%20Structure%20%28by%20ref%29))
  (bind _returnvalue (Actor|GetComponentbyClass OtherActor "/Script/Engine.SplineComponent"))
  (bind _canattachrail (Variables|Default|GetcanAttachRail))
  ;[0.4399 0.6383 0.7969 0.5] Is On Rail
  (Utilities|FlowControl|DoOnce false
    (:Completed
      (switch Utilities|FlowControl|Switch|SwitchonPlayerWagon_ENUM "NewEnumerator0"
        (:NewEnumerator0
          (Development|PrintString "BEGIN OVERLAP RAIL" true true "(R=0.000000,G=0.660000,B=1.000000,A=1.000000)" 1e+01)
          (Development|PrintString (Utilities|String|Append "MODE" (Utilities|String|EnumtoString (Variables|Default|GetVehicleMode))) true true "(R=0.000000,G=0.660000,B=1.000000,A=1.000000)" 1e+01)
          (Development|PrintString (Utilities|String|Append "CAN ATTACH" (Utilities|String|ToString(Boolean) _canattachrail)) true true "(R=0.000000,G=0.660000,B=1.000000,A=1.000000)" 1e+01)
          (Variables|/Script/Engine.PrimitiveComponent|SetbGenerateOverlapEvents (Variables|Character|GetMesh) false)
          (if (Variables|Default|GetRailTickEnabled)
            (if _canattachrail
              (if (Actor|ActorHasTag OtherActor "Rail")
                (Utilities|IsValid _returnvalue
                  (:Is%20Valid
                    (CallFunction|AddMappingContext "/Game/Input/IMC_VehicleRail.IMC_VehicleRail")
                    (Variables|Default|SetVehicleMode "NewEnumerator1")
                    (Variables|Default|SetCurrent%20Spline%20Rail _returnvalue)
                    (Variables|Default|SetSplineLenght (Spline|GetSplineLength (Variables|Default|GetCurrent%20Spline%20Rail)))
                    (bind _returnvalue_2 (Physics|GetPhysicsLinearVelocity (Variables|Character|GetMesh) "None"))
                    (bind _output_get (Variables|Default|SetRail%20Speed (.X (Math|Vector|BreakVector _returnvalue_2))))
                    (Development|PrintString (Utilities|String|ToString(Float) _output_get) true true "(R=0.000000,G=0.660000,B=1.000000,A=1.000000)" 1e+01)
                    (if (not (> (.Z (Math|Vector|BreakVector _returnvalue_2)) 0.0))
                      (Variables|Default|SetDistanceOnRail (Class|SplineComponent|GetDistanceAlongSplineatLocation (Variables|Default|GetCurrent%20Spline%20Rail) (Transformation|GetWorldLocation (Variables|Default|GetRailDetector)) "World"))
                      (Physics|SetSimulatePhysics (Variables|Character|GetMesh) false)
                      (CallFunction|ChaosOff))))))))))))

(event Custom|Reset
  (bind _canattachrail (Variables|Default|GetcanAttachRail))
  ;[0.4399 0.6383 0.7969 0.5] Is On Rail
  (Utilities|FlowControl|DoOnce false) ; enters at Reset
)

(event Input|EnhancedActionEvents|EnhancedInputActionIA_Look_Mod
  (params (ActionValue :type Vector%202D%20Structure) (ElapsedSeconds :type Float%20%28double-precision%29) (TriggeredSeconds :type Float%20%28double-precision%29) (InputAction :type Input%20Action%20Object%20Reference :default "/Game/Input/Actions/IA_Look_Mod.IA_Look_Mod"))
  ;[0.2918 0.1714 0.005605] IA_Look
  (Pawn|Input|AddControllerYawInput (.x ActionValue))
  (Pawn|Input|AddControllerPitchInput (.y ActionValue)))

(event Input|EnhancedActionEvents|EnhancedInputActionIA_Throttle
  (params (ActionValue :type Float%20%28double-precision%29) (ElapsedSeconds :type Float%20%28double-precision%29) (TriggeredSeconds :type Float%20%28double-precision%29) (InputAction :type Input%20Action%20Object%20Reference :default "/Game/VehicleTemplate/Input/Actions/IA_Throttle.IA_Throttle"))
  ;[0.7188 0.4257 0.01295 0.5] IA_Throttle
  (:Triggered
    (switch Utilities|FlowControl|Switch|SwitchonPlayerWagon_ENUM (Variables|Default|GetVehicleMode) :!label _label
      (:NewEnumerator0
        (Class|ChaosVehicleMovementComponent|SetThrottleInput (Variables|Default|GetVehicleMovementComponent) ActionValue))))
  (:Completed
    (goto _label)))

(event Input|EnhancedActionEvents|EnhancedInputActionIA_Shoot
  (params (ActionValue :type Boolean) (ElapsedSeconds :type Float%20%28double-precision%29) (TriggeredSeconds :type Float%20%28double-precision%29) (InputAction :type Input%20Action%20Object%20Reference :default "/Game/Input/Actions/IA_Shoot.IA_Shoot"))
  ;[0.15 0.15 0.15 0.5] Shoot
  (if (> (Variables|Default|GetCantidadMisiles) 0.0)
    (Game|SpawnActorfromClass "/Game/Blueprints/Objects/BP_Misil.BP_Misil_C" (Math|Transform|MakeTransform (Transformation|GetSocketLocation (Variables|Character|GetMesh) "Brake") (Transformation|GetActorRotation) "1.000000,1.000000,1.000000") "Undefined" "MultiplyWithRoot" 0 0)
    (Variables|Default|SetCantidadMisiles 0.0)))

(event Input|EnhancedActionEvents|EnhancedInputActionIA_Turbo
  (params (ActionValue :type Boolean) (ElapsedSeconds :type Float%20%28double-precision%29) (TriggeredSeconds :type Float%20%28double-precision%29) (InputAction :type Input%20Action%20Object%20Reference :default "/Game/Input/Actions/IA_Turbo.IA_Turbo"))
  (bind _mesh (Variables|Character|GetMesh))
  (bind _returnvalue (Transformation|GetComponentVelocity _mesh))
  ;[0.15 0.15 0.15 0.5] Turbo
  (if (> (Variables|Default|GetCantidad%20Turbo) 0.0)
    (Physics|AddForce _mesh (Math|Vector|MakeVector (* (.x _returnvalue) 3.0) (* (.y _returnvalue) 3.0) (.z _returnvalue)) "None" false)
    (Variables|Default|SetCantidad%20Turbo (- (Variables|Default|GetCantidad%20Turbo) 1.0))))

(event Input|EnhancedActionEvents|EnhancedInputActionIA_Brake
  (params (ActionValue :type Float%20%28double-precision%29) (ElapsedSeconds :type Float%20%28double-precision%29) (TriggeredSeconds :type Float%20%28double-precision%29) (InputAction :type Input%20Action%20Object%20Reference :default "/Game/Input/Actions/IA_Brake.IA_Brake"))
  ;[0.2918 0.1714 0.005605] IA_Brake
  (:Triggered
    ;[0.7188 0.4257 0.01295 0.5] IA_Throttle
    (switch Utilities|FlowControl|Switch|SwitchonPlayerWagon_ENUM (Variables|Default|GetVehicleMode) :!label _label
      (:NewEnumerator0
        (Class|ChaosVehicleMovementComponent|SetBrakeInput (Variables|Default|GetVehicleMovementComponent) ActionValue))))
  (:Completed
    (goto _label)))

(event Input|EnhancedActionEvents|EnhancedInputActionIA_Steering
  (params (ActionValue :type Float%20%28double-precision%29) (ElapsedSeconds :type Float%20%28double-precision%29) (TriggeredSeconds :type Float%20%28double-precision%29) (InputAction :type Input%20Action%20Object%20Reference :default "/Game/Input/Actions/IA_Steering.IA_Steering"))
  ;[0.2087 0.1546 0.04784] IA_Steering
  (:Triggered
    (switch Utilities|FlowControl|Switch|SwitchonPlayerWagon_ENUM (Variables|Default|GetVehicleMode) :!label _label
      (:NewEnumerator0
        (Class|ChaosVehicleMovementComponent|SetSteeringInput (Variables|Default|GetVehicleMovementComponent) ActionValue)
        (CallFunction|ParachuteSteering ActionValue))))
  (:Completed
    (goto _label)))

(event Input|EnhancedActionEvents|EnhancedInputActionIA_Light
  (params (ActionValue :type Boolean) (ElapsedSeconds :type Float%20%28double-precision%29) (TriggeredSeconds :type Float%20%28double-precision%29) (InputAction :type Input%20Action%20Object%20Reference :default "/Game/Input/Actions/IA_Light.IA_Light"))
  (bind _light (Variables|Default|GetLight))
  (bind _mesh (Variables|Character|GetMesh))
  ;[0.9751 1 0.3698 0.5] IA_Light
  (:Completed
    (Utilities|FlowControl|FlipFlop
      (:A
        (Rendering|SetVisibility _light true false)
        (Rendering|Material|SetVectorParameterValueonMaterials _mesh "Emissive Color" "1.000000,0.600000,0.000000"))
      (:B
        (Rendering|SetVisibility _light false false)
        (Rendering|Material|SetVectorParameterValueonMaterials _mesh "Emissive Color" "0, 0, 0")))))

(event Input|EnhancedActionEvents|EnhancedInputActionIA_Parachute
  (params (ActionValue :type Boolean) (ElapsedSeconds :type Float%20%28double-precision%29) (TriggeredSeconds :type Float%20%28double-precision%29) (InputAction :type Input%20Action%20Object%20Reference :default "/Game/Input/Actions/IA_Parachute.IA_Parachute"))
  (bind _returnvalue (Transformation|GetActorLocation))
  ;[0.025 0.1102 0.15 0.5] IA_Parachute
  (:Started
    ;;[0.15 0.15 0.15 0.5] Distance to ground
    (bind _outhit (Collision|LineTraceByChannel _returnvalue (+ _returnvalue (* (Math|Vector|GetUpVector (Variables|Character|GetMesh)) -1e+04)) "TraceTypeQuery1" false 0 "ForDuration"))
    (if (> (.Distance (Collision|BreakHitResult _outhit)) 0.0)
      (Variables|Default|SetIsOnAir true)
      (if (> (.Distance (Collision|BreakHitResult _outhit)) 2e+02)
        (Variables|Default|SetIsParachuteDeployed true)
        (Rendering|SetVisibility (Variables|Default|GetParachute) true false)
        ;;[0.15 0.15 0.15 0.5] Deploying Initial up force
        (bind _returnvalue_2 (Physics|GetPhysicsLinearVelocity (Variables|Character|GetMesh) "None"))
        (Physics|AddForce (Variables|Character|GetMesh) (+ (Transformation|GetActorLocation) (Math|Vector|MakeVector 0.0 0.0 (Math|Float|Absolute(Float) (* (.Z (Math|Vector|BreakVector _returnvalue_2)) 5e+01)))) "None" false))
      (else
        (Variables|Default|SetIsOnAir false))))
  (:Canceled
    (Variables|Default|SetIsParachuteDeployed false :!label _label)
    (Rendering|SetVisibility (Variables|Default|GetParachute) false false)
    (Class|PrimitiveComponent|SetAngularDamping (Variables|Character|GetMesh) 0.0))
  (:Completed
    (goto _label)))

(event Input|EnhancedActionEvents|EnhancedInputActionIA_Jump
  (params (ActionValue :type Boolean) (ElapsedSeconds :type Float%20%28double-precision%29) (TriggeredSeconds :type Float%20%28double-precision%29) (InputAction :type Input%20Action%20Object%20Reference :default "/Game/Input/Actions/IA_Jump.IA_Jump"))
  (bind _returnvalue (Transformation|GetActorLocation))
  ;[0.09219 0.15 0.1212 0.5] IA_Jump
  (:Started
    ;;[0.15 0.15 0.15 0.5] Can Jump?
    (bind _outhit (Collision|LineTraceByChannel _returnvalue (+ _returnvalue (* (Math|Vector|GetUpVector (Variables|Character|GetMesh)) -2e+02)) "TraceTypeQuery1" false 0 "ForDuration"))
    (if (not (> (.Distance (Collision|BreakHitResult _outhit)) 0.0))
      (switch Utilities|FlowControl|Switch|SwitchonPlayerWagon_ENUM (Variables|Default|GetVehicleMode)
        (:NewEnumerator0
          ;;[0.15 0.15 0.15 0.5] Wheels Jump
          (Physics|AddImpulse (Variables|Character|GetMesh) (* (Transformation|GetActorUpVector) 4e+02) "None" true))
        (:NewEnumerator1
          (if (not (Variables|Default|GetExit%20Rail))
            (CallFunction|ExitRail)
            ;;[0.15 0.15 0.15 0.5] Evitar reenganche de vía
            (Variables|Default|SetcanAttachRail false)
            (Utilities|FlowControl|Delay 0.2)
            (Variables|Default|SetcanAttachRail true)))))))

(event Input|EnhancedActionEvents|EnhancedInputActionIA_MoveForwardRail
  (params (ActionValue :type Float%20%28double-precision%29) (ElapsedSeconds :type Float%20%28double-precision%29) (TriggeredSeconds :type Float%20%28double-precision%29) (InputAction :type Input%20Action%20Object%20Reference :default "/Game/Input/Actions/IA_MoveForwardRail.IA_MoveForwardRail"))
  ;[0.15 0.15 0.15 0.5] IMC_VehicleRail
  (:Triggered
    (switch Utilities|FlowControl|Switch|SwitchonPlayerWagon_ENUM (Variables|Default|GetVehicleMode) :!label _label
      (:NewEnumerator1
        (Variables|Default|SetRailInput ActionValue))))
  (:Completed
    (goto _label)))

(event Input|EnhancedActionEvents|EnhancedInputActionIA_BrakeRail
  (params (ActionValue :type Float%20%28double-precision%29) (ElapsedSeconds :type Float%20%28double-precision%29) (TriggeredSeconds :type Float%20%28double-precision%29) (InputAction :type Input%20Action%20Object%20Reference :default "/Game/Input/Actions/IA_BrakeRail.IA_BrakeRail"))
  ;[0.15 0.15 0.15 0.5] IMC_VehicleRail
  (:Triggered
    (switch Utilities|FlowControl|Switch|SwitchonPlayerWagon_ENUM (Variables|Default|GetVehicleMode) :!label _label
      (:NewEnumerator1
        (Variables|Default|SetRailInput ActionValue))))
  (:Completed
    (goto _label)))

(event Input|EnhancedActionEvents|EnhancedInputActionIA_LateralJump
  (params (ActionValue :type Float%20%28double-precision%29) (ElapsedSeconds :type Float%20%28double-precision%29) (TriggeredSeconds :type Float%20%28double-precision%29) (InputAction :type Input%20Action%20Object%20Reference :default "/Game/Input/Actions/IA_LateralJump.IA_LateralJump"))
  ;[0.15 0.15 0.15 0.5] IMC_VehicleRail
  (:Triggered
    (switch Utilities|FlowControl|Switch|SwitchonPlayerWagon_ENUM (Variables|Default|GetVehicleMode) :!label _label
      (:NewEnumerator1
        (Variables|Default|SetSteerinInputRail ActionValue))))
  (:Completed
    (goto _label)))

(event Game|Damage|EventAnyDamage
  (params (Damage :type Float%20%28single-precision%29) (DamageType :type Damage%20Type%20Object%20Reference) (InstigatedBy :type Controller%20Object%20Reference) (DamageCauser :type Actor%20Object%20Reference))
  ;[0.15 0.15 0.15 0.5] Daño
  (if (> (Variables|Default|GetLife) 0)
    (bind _output_get (Variables|Default|SetLife (- (Variables|Default|GetLife) Damage)))
    (if (<= _output_get 0)
      (UserInterface|CreateWidget "/Game/Levels/HUD/WBP_GameOver.WBP_GameOver_C" (Game|GetPlayerController 1))
      (Input|DisableInput (Game|GetPlayerController 1))
      (Utilities|FlowControl|Delay 3.0)
      (Pawn|UnPossess (Pawn|GetLocalViewingPlayerController)))))

(event Collision|EventActorBeginOverlap
  (params (OtherActor :type Actor%20Object%20Reference)))

(event EventTick
  (params (DeltaSeconds :type Float%20%28single-precision%29))
  ;[0.15 0.05703 0.05703 0.5] Event Tick
  (switch Utilities|FlowControl|Switch|SwitchonPlayerWagon_ENUM (Variables|Default|GetVehicleMode)
    (:NewEnumerator0
      (CallFunction|Reset)
      (Variables|Default|SetExit%20Rail false)
      (if (Variables|Default|GetIsOnAir)
        (if (Variables|Default|GetIsParachuteDeployed)
          ;;[0.15 0.15 0.15 0.5] Parachute Deployed
          (CallFunction|SetVisibilityVisualMesh false true)
          (CallFunction|SetFieldOfView 9e+01 1.1e+02)
          (CallFunction|SetParachuteCamera "30.000000,0.000000,0.000000" "0.000000,0.000000,-100.000000")
          (else
            (CallFunction|SetVisibilityVisualMesh true false)
            (CallFunction|SetFieldOfView 1.1e+02 9e+01)
            (CallFunction|SetParachuteCamera "0, 0, 0" "0, 0, 0")))
        (CallFunction|LiftParachute)))
    (:NewEnumerator1
      (if (not (Variables|Default|GetExit%20Rail))
        (Utilities|IsValid (Variables|Default|GetCurrent%20Spline%20Rail)
          (:Is%20Valid
            (CallFunction|SetRailSpeed)
            (CallFunction|DistanceonRailCalc)
            ;;[0.15 0.15 0.15 0.5] End of Rail?
            (if (>= (Variables|Default|GetDistanceOnRail) (Variables|Default|GetSplineLenght))
              (Variables|Default|SetExit%20Rail false)
              (CallFunction|ExitRail)
              (else
                (CallFunction|RailMovement))))
          (:Is%20Not%20Valid
            (Variables|Default|SetExit%20Rail false)))))))

(event EventBeginPlay
  ;[0.15 0.15 0.15 0.5] HUD
  (bind _returnvalue (UserInterface|CreateWidget "/Game/Levels/HUD/WBP_Interfaz.WBP_Interfaz_C" (Game|GetPlayerController 1) (Variables|Default|GetWagon%20Info)))
  (UserInterface|Viewport|AddtoViewport _returnvalue 0)
  ;[0.15 0 0.001071 0.5] IMC
  (CallFunction|AddMappingContext "/Game/Input/IMC_Vehicle.IMC_Vehicle"))

(fn ConstructionScript)

(fn AddMappingContext
  (params (MappingContext :type Input%20Mapping%20Context%20Object%20Reference))
  (bind _asplayer_controller (Utilities|Casting|CastToPlayerController (Pawn|GetController)))
  (Input|AddMappingContext (PlayerController|LocalPlayerSubsystems|GetEnhancedInputLocalPlayerSubsystem _asplayer_controller) MappingContext 0 "(bIgnoreAllPressedKeysUntilRelease=True,bForceImmediately=False,bNotifyUserSettings=False)"))

(fn LiftParachute
  (bind _visualmeshparachute (Variables|Default|GetVisualMeshParachute))
  (bind _springarm (Variables|Default|GetSpringArm))
  (bind _relativerotation (Variables|/Script/Engine.SceneComponent|GetRelativeRotation _springarm))
  (Utilities|FlowControl|Sequence
    (:then_0
      ;[0.15 0.15 0.15 0.5] Planeo
      (bind _returnvalue (Physics|GetPhysicsLinearVelocity (Variables|Character|GetMesh) "None"))
      ;[0.15 0.15 0.15 0.5] Normaliza valor inclinación
      (Utilities|FlowControl|Sequence
        (:then_0
          (bind _output_get (Variables|Default|SetLateralSpeed (.Y (Math|Vector|BreakVector (Math|Vector|UnrotateVector _returnvalue (Transformation|GetActorRotation))))))
          (Variables|Default|SetNormalizedLateral (/ (Math|Float|Clamp(Float) _output_get -1.0) (Variables|Default|GetMaxLateralSpeedForBank))))
        (:then_1
          (Physics|AddForce (Variables|Character|GetMesh) (+ (Math|Vector|MakeVector 0.0 0.0 (Math|Float|Absolute(Float) (* (.Z (Math|Vector|BreakVector _returnvalue)) (Variables|Default|GetAirLiftForce)))) (* (Transformation|GetActorForwardVector) (Variables|Default|GetGlide))) "None" false))))
    (:then_1
      (Class|PrimitiveComponent|SetAngularDamping (Variables|Character|GetMesh) 3.0)
      (Class|PrimitiveComponent|SetLinearDamping (Variables|Character|GetMesh) 0.5))
    (:then_2
      ;[0.15 0.15 0.15 0.5] Inclinación
      (Transformation|SetRelativeRotation _visualmeshparachute (Math|Interpolation|RInterpTo (Variables|/Script/Engine.SceneComponent|GetRelativeRotation _visualmeshparachute) (Math|Rotator|MakeRotator (Variables|Default|GetTargetRoll) 0.0 0.0) (Utilities|Time|GetWorldDeltaSeconds) (Variables|Default|GetBankInterpSpeed)) false false))
    (:then_3
      ;[0.15 0.15 0.15 0.5] Inclinación Cámara
      (Transformation|SetRelativeRotation (Variables|Default|GetSpringArm) (Math|Rotator|MakeRotator (* (Math|Interpolation|FInterpTo (.roll _relativerotation) (Math|Float|MapRangeClamped (.Z (Math|Vector|BreakVector (Physics|GetPhysicsAngularVelocityinDegrees (Variables|Character|GetMesh) "None"))) -1.8e+02 1.8e+02 -2e+01 2e+01) (Utilities|Time|GetWorldDeltaSeconds) 3.0) 2.0) (.pitch _relativerotation) (.yaw _relativerotation)) false false))
    (:then_4)))

(fn ParachuteSteering
  (params (Action%20Value :type Float%20%28double-precision%29))
  (bind _mesh (Variables|Character|GetMesh))
  (if (Variables|Default|GetIsParachuteDeployed)
    (bind _output_get (Variables|Default|SetTargetRoll (* (Variables|Default|GetBankAngleMax) Action%20Value)))
    (if (== Action%20Value 0.0)
      (Variables|Default|SetTargetRoll 0.0)
      (Utilities|FlowControl|Sequence
        (:then_0
          (Rendering|SetVisibility (Variables|Character|GetMesh) true false)
          (bind _returnvalue (Physics|GetPhysicsLinearVelocity (Variables|Character|GetMesh) "None" :!label _label))
          (if (< (Math|Float|Absolute(Float) (.Y (Math|Vector|BreakVector _returnvalue))) (Variables|Default|GetMaxAirLateralSpeed))
            (Physics|AddForce _mesh (+ _returnvalue (* (* (Transformation|GetActorRightVector) Action%20Value) (Variables|Default|GetAirLateralForce))) "None" false)
            (Class|PrimitiveComponent|AddAngularImpulseinDegrees _mesh (Math|Vector|ClampVectorSize (Math|Vector|MakeVector 0.0 0.0 (* Action%20Value 5.0)) -1.0 1.0) "None" true)))
        (:then_1
          (Rendering|SetVisibility (Variables|Default|GetVisualMesh) false false)))
      (else
        (Variables|Default|SetTargetRoll _output_get)
        (Utilities|FlowControl|Sequence
          (:then_0
            (Rendering|SetVisibility (Variables|Character|GetMesh) false false)
            (goto _label))
          (:then_1
            (Rendering|SetVisibility (Variables|Default|GetVisualMesh) true false)))))))

(fn Parada)

(fn SetVisibilityVisualMesh
  (params (MeshVisibility :type Boolean) (VirtualMesh%20Visibility :type Boolean))
  (Rendering|SetVisibility (Variables|Character|GetMesh) MeshVisibility false)
  (Rendering|SetVisibility (Variables|Default|GetVisualMesh) VirtualMesh%20Visibility false))

(fn SetFieldOfView
  (params (Current :type Float%20%28double-precision%29) (Target :type Float%20%28double-precision%29))
  (Camera|SetFieldOfView (Variables|Default|GetCamera) (Math|Interpolation|FInterpTo Current Target (Utilities|Time|GetWorldDeltaSeconds) 3.0)))

(fn SetParachuteCamera
  (params (NewRotation :type Rotator) (NewLocation :type Vector))
  (Transformation|SetRelativeRotation (Variables|Default|GetSpringArm) NewRotation false false)
  (Transformation|SetRelativeLocation (Variables|Default|GetCamera) NewLocation false false))

(fn ExitRail
  (bind _mesh (Variables|Character|GetMesh))
  (bind _rail_speed (Variables|Default|GetRail%20Speed))
  (bind _returnvalue (Math|Vector|GetForwardVector _mesh))
  (bind _returnvalue_2 (* _returnvalue _rail_speed))
  (Variables|Default|SetRailTickEnabled true)
  (Development|PrintString "EXIT RAIL CALLED" true true "(R=0.000000,G=0.660000,B=1.000000,A=1.000000)" 1e+01)
  (Variables|Default|SetCurrent%20Spline%20Rail 0)
  (Physics|SetSimulatePhysics (Variables|Character|GetMesh) true)
  (Physics|SetPhysicsLinearVelocity (Variables|Character|GetMesh) _returnvalue_2 false "None")
  (Development|PrintString (Utilities|String|Append "Actual Velocity:" (Utilities|String|ToString(Vector) _returnvalue_2)) true true "(R=0.000000,G=0.660000,B=1.000000,A=1.000000)" 1e+01)
  (Collision|SetCollisionEnabled (Variables|Character|GetMesh) "QueryAndPhysics")
  (CallFunction|Chaoson)
  (CallFunction|JumponRailImpulse)
  (Variables|/Script/Engine.PrimitiveComponent|SetbGenerateOverlapEvents (Variables|Character|GetMesh) true)
  (Components|Tick|SetComponentTickEnabled (Variables|Character|GetMesh) true)
  (Development|PrintString (Utilities|String|Append "Initial Mode" (Utilities|String|EnumtoString (Variables|Default|GetVehicleMode))) true true "(R=0.000000,G=0.660000,B=1.000000,A=1.000000)" 1e+01)
  (Variables|Default|SetVehicleMode "NewEnumerator0")
  (Components|Movement|SetUpdatedComponent (Variables|Default|GetVehicleMovementComponent) (Variables|Character|GetMesh))
  (Components|Movement|StopMovementImmediately (Variables|Default|GetVehicleMovementComponent))
  (Development|PrintString (Utilities|String|EnumtoString (Variables|Default|GetVehicleMode)) true true "(R=0.000000,G=0.660000,B=1.000000,A=1.000000)" 5.0)
  (CallFunction|AddMappingContext "/Game/Input/IMC_Vehicle.IMC_Vehicle")
  (CallFunction|RemoveMappingContext "/Game/Input/IMC_VehicleRail.IMC_VehicleRail"))

(fn ChaosOff
  (Components|Movement|StopMovementImmediately (Variables|Default|GetVehicleMovementComponent))
  (Components|Movement|SetUpdatedComponent (Variables|Default|GetVehicleMovementComponent) 0)
  (Components|Tick|SetComponentTickEnabled (Variables|Character|GetMesh) false))

(fn Chaoson
  (Class|PrimitiveComponent|WakeRigidBody (Variables|Character|GetMesh) "None")
  (Components|Movement|SetUpdatedComponent (Variables|Default|GetVehicleMovementComponent) (Variables|Character|GetMesh))
  (Components|Tick|SetComponentTickEnabled (Variables|Character|GetMesh) true))

(fn SetRailSpeed
  (bind _output_get (Variables|Default|SetRail%20Speed (* (Math|Float|Clamp(Float) (+ (Variables|Default|GetRail%20Speed) (* (* (Variables|Default|GetRailInput) (Variables|Default|GetRailAccel)) (Utilities|Time|GetWorldDeltaSeconds))) (* (+ (Variables|Default|GetRail%20Speed) (* (* (Variables|Default|GetRailInput) (Variables|Default|GetRailAccel)) (Utilities|Time|GetWorldDeltaSeconds))) -1.0) (Variables|Default|GetRailMaxSpeed)) (Variables|Default|GetRailDrag))))
  (return _output_get))

(fn JumponRailImpulse
  (bind _returnvalue (Physics|GetPhysicsLinearVelocity (Variables|Character|GetMesh) "None"))
  (Physics|AddImpulse (Variables|Character|GetMesh) (+ (* (Transformation|GetActorUpVector) 3e+02) (+ (* _returnvalue 0.6) (* (Transformation|GetActorRightVector) (* (Variables|Default|GetJumpLateral%20Force) (Variables|Default|GetSteerinInputRail))))) "None" true))

(fn RailMovement
  (bind _current_spline_rail (Variables|Default|GetCurrent%20Spline%20Rail))
  (bind _distanceonrail (Variables|Default|GetDistanceOnRail))
  (bind _returnvalue (Spline|GetTransformatDistanceAlongSpline _current_spline_rail _distanceonrail "World" false))
  (Transformation|SetWorldLocationAndRotation (Variables|Character|GetMesh) (+ (.location _returnvalue) "0.000000,0.000000,-3.000000") (.rotation _returnvalue) false true))

(fn DistanceonRailCalc
  (Variables|Default|SetDistanceOnRail (+ (Variables|Default|GetDistanceOnRail) (* (Variables|Default|GetRail%20Speed) (Utilities|Time|GetWorldDeltaSeconds)))))

(fn RemoveMappingContext
  (params (MappingContext :type Input%20Mapping%20Context%20Object%20Reference))
  (bind _asplayer_controller (Utilities|Casting|CastToPlayerController (Pawn|GetController)))
  (Input|RemoveMappingContext (PlayerController|LocalPlayerSubsystems|GetEnhancedInputLocalPlayerSubsystem _asplayer_controller) MappingContext "(bIgnoreAllPressedKeysUntilRelease=True,bForceImmediately=False,bNotifyUserSettings=False)"))

(fn CogerMonedas
  (Variables|Default|SetMonedas (+ (Variables|Default|GetMonedas) 1)))

(fn CogerTurbo
  (Variables|Default|SetCantidad%20Turbo (+ (Variables|Default|GetCantidad%20Turbo) 1e+01)))

(fn CogerMisil
  (Variables|Default|SetCantidadMisiles (+ (Variables|Default|GetCantidadMisiles) 1.0)))