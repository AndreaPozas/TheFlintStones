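; BP_Vagoneta is a wagon with a CharacterMovement component that rides along the spline of a Path_BP actor.
; Each Tick it accumulates distance from MaxWalkSpeed, looks up the path, and snaps its location and rotation to that spline point.
; On looping paths it calls Parada past the end and prints a test station message shortly before.
; Parada is empty; the stop, wait and restart logic is disconnected.
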(event Custom|Parada)

(event EventBeginPlay)

(event Collision|EventActorBeginOverlap
  (params (OtherActor :type Actor%20Object%20Reference)))

(event EventTick
  (params (DeltaSeconds :type Float%20%28single-precision%29))
  (Utilities|FlowControl|Sequence
    (:then_0
      (Variables|Default|SetDistancia%20Recorrido (+ (* DeltaSeconds (Variables|/Script/Engine.CharacterMovementComponent|GetMaxWalkSpeed (Variables|Character|GetCharacterMovement))) (Variables|Default|GetDistancia%20Recorrido)))
      (bind _returnvalue (Actor|GetActorOfClass "/Game/Blueprints/Path_BP.Path_BP_C"))
      (Transformation|SetActorRelativeTransform (Math|Transform|MakeTransform (.location (Spline|GetTransformatDistanceAlongSpline (Variables|/Game/Blueprints/Path_BP.Path_BP_C|GetSpline _returnvalue) (Variables|Default|GetDistancia%20Recorrido) "World" false)) (.rotation (Spline|GetTransformatDistanceAlongSpline (Variables|/Game/Blueprints/Path_BP.Path_BP_C|GetSpline _returnvalue) (Variables|Default|GetDistancia%20Recorrido) "World" false)) (Transformation|GetActorScale3D)) false false)
      (if (Variables|/Game/Blueprints/Path_BP.Path_BP_C|GetLoop _returnvalue)
        (if (> (Variables|Default|GetDistancia%20Recorrido) (Spline|GetSplineLength (Variables|/Game/Blueprints/Path_BP.Path_BP_C|GetSpline _returnvalue)))
          (CallFunction|Parada)
          (elif (> (Variables|Default|GetDistancia%20Recorrido) (- (Spline|GetSplineLength (Variables|/Game/Blueprints/Path_BP.Path_BP_C|GetSpline _returnvalue)) 5e+02))
            (Development|PrintText "Prueba Estación")))))))

(fn ConstructionScript)