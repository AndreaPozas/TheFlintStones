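; Construction path Blueprint, named as a long rail, that lays a mesh along an editable spline.
; The construction script divides the spline length by MeshSize and adds one spline mesh component per whole segment, using the Mesh variable with query and physics collision.
; Each segment takes local-space positions from the spline, with tangents clamped to MeshSize to limit distortion.
; The event graph is empty, so the actor has no runtime logic.
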(event EventBeginPlay)

(event Collision|EventActorBeginOverlap
  (params (OtherActor :type Actor%20Object%20Reference)))

(event EventTick
  (params (DeltaSeconds :type Float%20%28single-precision%29)))

(fn ConstructionScript
  (bind _spline (Variables|Default|GetSpline))
  (bind _mesh_size (Variables|Default|GetMesh%20Size))
  (for _index (range 0 (- (Math|Float|Truncate (/ (Spline|GetSplineLength (Variables|Default|GetSpline)) (Variables|Default|GetMesh%20Size))) 1))
    (bind _returnvalue (AddComponent|AddSplineMeshComponent false))
    (SplineMesh|SetStartandEnd _returnvalue (Spline|GetLocationatDistanceAlongSpline _spline (* _index _mesh_size) "Local") (Math|Vector|ClampVectorSize (Spline|GetTangentatDistanceAlongSpline _spline (* _index _mesh_size) "Local") 0.0 _mesh_size) (Spline|GetLocationatDistanceAlongSpline _spline (+ (* _index _mesh_size) _mesh_size) "Local") (Math|Vector|ClampVectorSize (Spline|GetTangentatDistanceAlongSpline _spline (+ (* _index _mesh_size) _mesh_size) "Local") 0.0 _mesh_size) true :!class /Script/Engine.SplineMeshComponent)
    (Collision|SetCollisionEnabled _returnvalue "QueryAndPhysics")
    (Components|StaticMesh|SetStaticMesh _returnvalue (Variables|Default|GetMesh))))